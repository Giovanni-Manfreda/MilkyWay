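; BP_SpaceShip is a physics-driven spaceship that yaws, pitches, rolls and moves along its forward vector.
; Look and roll events apply mass-independent torque around the mesh's local axes, scaled by per-axis power values.
; MoveSpaceShip eases thrust toward a max or min target and overwrites linear velocity with it.
; StartDeceleration toggles a looping frame-delta timer that eases thrust back to normal, updating velocity the same way.
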(event Custom|Thrust%20Deceleraation
  (bind _output_get (Variables|Default|SetCurrent%20Thrust (Math|Interpolation|FInterpTo (Variables|Default|GetCurrent%20Thrust) (Variables|ToolKit|GetNormal%20Thrust) (Utilities|Time|GetWorldDeltaSeconds) 3.0)))
  (Physics|SetPhysicsLinearVelocity (Variables|Default|GetSM_SpaceBlockout) (* _output_get (Math|Vector|GetForwardVector (Variables|Default|GetSM_SpaceBlockout))) false "None"))

(event EventBeginPlay)

(event Collision|EventActorBeginOverlap
  (params (OtherActor :type Actor%20Object%20Reference)))

(event EventTick
  (params (DeltaSeconds :type Float%20%28single-precision%29)))

(event EventLookRight&Left
  (params (Input%20Values :type Float%20%28double-precision%29))
  (Class|PrimitiveComponent|AddTorqueinDegrees (Variables|Default|GetSM_SpaceBlockout) (* (* Input%20Values (Variables|ToolKit|GetLook%20Right%20Left%20Power)) (Math|Vector|GetUpVector (Variables|Default|GetSM_SpaceBlockout))) "None" true))

(event EventLookTop&Down
  (params (Input%20Values :type Float%20%28double-precision%29))
  (Class|PrimitiveComponent|AddTorqueinDegrees (Variables|Default|GetSM_SpaceBlockout) (* (* Input%20Values (Variables|ToolKit|GetLook%20Top%20Down%20Power)) (Math|Vector|GetRightVector (Variables|Default|GetSM_SpaceBlockout))) "None" true))

(event EventRollRight&Left
  (params (Input%20Value :type Float%20%28double-precision%29))
  (Class|PrimitiveComponent|AddTorqueinDegrees (Variables|Default|GetSM_SpaceBlockout) (* (* Input%20Value (Variables|ToolKit|GetRoll%20Right%20Left%20Power)) (Math|Vector|GetForwardVector (Variables|Default|GetSM_SpaceBlockout))) "None" true))

(event EventMoveSpaceShip
  (params (Input%20Value :type Boolean))
  (bind _output_get (Variables|Default|SetCurrent%20Thrust (Math|Interpolation|FInterpTo (Variables|Default|GetCurrent%20Thrust) (Math|Float|SelectFloat (Variables|ToolKit|GetMax%20Thrust) (Variables|ToolKit|GetMin%20Thrust) Input%20Value) (Utilities|Time|GetWorldDeltaSeconds) 1.0)))
  (Physics|SetPhysicsLinearVelocity (Variables|Default|GetSM_SpaceBlockout) (* _output_get (Math|Vector|GetForwardVector (Variables|Default|GetSM_SpaceBlockout))) false "None"))

(event EventStartDeceleration
  (params (Decelerate? :type Boolean))
  (if Decelerate?
    (bind _returnvalue (Utilities|Time|SetTimerbyEvent (delegate Custom|Thrust%20Deceleraation) (Utilities|Time|GetWorldDeltaSeconds) true))
    (Variables|Default|SetTImer%20Handler%20Deceleration _returnvalue)
    (else
      (Utilities|Time|ClearandInvalidateTimerbyHandle (Variables|Default|GetTImer%20Handler%20Deceleration)))))

(fn ConstructionScript)