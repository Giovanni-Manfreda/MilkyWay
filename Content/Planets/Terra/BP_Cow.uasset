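; Cow actor on planet Terra that gets pulled into the player's spaceship and disappears.
; Sphere overlap with the player pawn sets the target, and ending the overlap clears it.
; While targeted, Tick moves the cow to the pawn via VInterpTo with a fixed delta time and no set speed, effectively snapping.
; Each pull also shrinks the Cube component, destroying the actor at zero scale.
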(event OnComponentBeginOverlap(Sphere)
  (params (OverlappedComponent :type Primitive%20Component%20Object%20Reference) (OtherActor :type Actor%20Object%20Reference) (OtherComp :type Primitive%20Component%20Object%20Reference) (OtherBodyIndex :type Integer) (bFromSweep :type Boolean) (SweepResult :type Hit%20Result%20Structure%20%28by%20ref%29))
  (Development|PrintString "Hello")
  (if (== OtherActor (Game|Player|GetPlayerPawn 0))
    (Variables|Default|SetTarget%20Actor OtherActor)
    (CallFunction|PullTowardsTarget)))

(event OnComponentEndOverlap(Sphere)
  (params (OverlappedComponent :type Primitive%20Component%20Object%20Reference) (OtherActor :type Actor%20Object%20Reference) (OtherComp :type Primitive%20Component%20Object%20Reference) (OtherBodyIndex :type Integer))
  (if (== OtherActor (Game|Player|GetPlayerPawn 0))
    (Variables|Default|SetTarget%20Actor 0)))

(event Custom|PullTowardsTarget
  (bind _cube (Variables|Default|GetCube))
  (bind _spaceshiplocation (CallFunction|GetSpaceshipLocation))
  (CallFunction|CalculateFinalDestination _spaceshiplocation)
  (Transformation|SetRelativeScale3D _cube (- (Variables|/Script/Engine.SceneComponent|GetRelativeScale3D _cube) "0.020000,0.020000,0.020000"))
  (if (<= (.x (Variables|/Script/Engine.SceneComponent|GetRelativeScale3D _cube)) 0.0)
    (Actor|DestroyActor)))

(event EventBeginPlay)

(event Collision|EventActorBeginOverlap
  (params (OtherActor :type Actor%20Object%20Reference)))

(event EventTick
  (params (DeltaSeconds :type Float%20%28single-precision%29))
  (Variables|Default|GetTarget%20Actor
    (:then
      (CallFunction|PullTowardsTarget))
    (:else)))

(fn ConstructionScript)

(fn GetSpaceshipLocation
  (return (Transformation|GetActorLocation (Game|Player|GetPlayerPawn 0))))

(fn CalculateFinalDestination
  (params (spaceshipLocation :type Vector))
  (Transformation|SetActorLocation (Math|Interpolation|VInterpTo (Transformation|GetActorLocation) spaceshipLocation 5.0 0.0) false false))