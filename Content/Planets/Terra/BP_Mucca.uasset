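; BP_Mucca is a cow actor on the Terra planet that gets pulled toward the spaceship, shrinking until it disappears.
; Its Sphere overlap events store the BP_SpaceShip reference and toggle the follow flag on entry and exit.
; While following, Tick eases the actor toward the ship with a swept VInterpTo move, shrinks the mesh by a frame-rate-dependent fixed step, and destroys the actor at zero scale.
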(event OnComponentBeginOverlap(Sphere)
  (params (OverlappedComponent :type Primitive%20Component%20Object%20Reference) (OtherActor :type Actor%20Object%20Reference) (OtherComp :type Primitive%20Component%20Object%20Reference) (OtherBodyIndex :type Integer) (bFromSweep :type Boolean) (SweepResult :type Hit%20Result%20Structure%20%28by%20ref%29))
  (bind _asbp_space_ship (Utilities|Casting|CastToBP_SpaceShip OtherActor))
  (Variables|Default|SetSpaceShipRef _asbp_space_ship)
  (Variables|Default|SetbSeguiSpaceship true))

(event OnComponentEndOverlap(Sphere)
  (params (OverlappedComponent :type Primitive%20Component%20Object%20Reference) (OtherActor :type Actor%20Object%20Reference) (OtherComp :type Primitive%20Component%20Object%20Reference) (OtherBodyIndex :type Integer))
  (bind _asbp_space_ship (Utilities|Casting|CastToBP_SpaceShip OtherActor))
  (Variables|Default|SetSpaceShipRef _asbp_space_ship)
  (Variables|Default|SetbSeguiSpaceship false))

(event EventBeginPlay)

(event Collision|EventActorBeginOverlap
  (params (OtherActor :type Actor%20Object%20Reference)))

(event EventTick
  (params (DeltaSeconds :type Float%20%28single-precision%29))
  (bind _staticmesh (Variables|Default|GetStaticMesh))
  (if (Variables|Default|GetbSeguiSpaceship)
    (Transformation|SetActorLocation (Math|Interpolation|VInterpTo (Transformation|GetActorLocation) (Transformation|GetActorLocation (Variables|Default|GetSpaceShipRef)) DeltaSeconds 0.5) true false)
    (Transformation|SetRelativeScale3D _staticmesh (- (Variables|/Script/Engine.SceneComponent|GetRelativeScale3D _staticmesh) "0.010000,0.010000,0.010000"))
    (if (<= (.x (Variables|/Script/Engine.SceneComponent|GetRelativeScale3D _staticmesh)) 0.0)
      (Actor|DestroyActor))))

(fn ConstructionScript)