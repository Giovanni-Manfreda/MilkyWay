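; PC_SpaceShip is the player controller for flying a spaceship, adding the IMC_Spaceship Enhanced Input context on BeginPlay.
; It forwards look, roll and move input to the controlled pawn through interface messages, reducing movement to a boolean for a positive value.
; Starting move input cancels deceleration and completing it starts deceleration.
; A Tab key press creates a new quest log widget and adds it to the viewport.
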(event Input|EnhancedActionEvents|EnhancedInputActionIA_LookLeftRight
  (params (ActionValue :type Float%20%28double-precision%29) (ElapsedSeconds :type Float%20%28double-precision%29) (TriggeredSeconds :type Float%20%28double-precision%29) (InputAction :type Input%20Action%20Object%20Reference :default "/Game/GameManager/Input_SpaceShip/IA_LookLeftRight.IA_LookLeftRight"))
  (Class|BPISpaceShip|LookRight&Left(Message) (Pawn|GetControlledPawn) ActionValue))

(event Input|EnhancedActionEvents|EnhancedInputActionIA_LookUpDown
  (params (ActionValue :type Float%20%28double-precision%29) (ElapsedSeconds :type Float%20%28double-precision%29) (TriggeredSeconds :type Float%20%28double-precision%29) (InputAction :type Input%20Action%20Object%20Reference :default "/Game/GameManager/Input_SpaceShip/IA_LookUpDown.IA_LookUpDown"))
  (Class|BPISpaceShip|LookTop&Down(Message) (Pawn|GetControlledPawn) ActionValue))

(event Input|EnhancedActionEvents|EnhancedInputActionIA_Roll
  (params (ActionValue :type Float%20%28double-precision%29) (ElapsedSeconds :type Float%20%28double-precision%29) (TriggeredSeconds :type Float%20%28double-precision%29) (InputAction :type Input%20Action%20Object%20Reference :default "/Game/GameManager/Input_SpaceShip/IA_Roll.IA_Roll"))
  (Class|BPISpaceShip|RollRight&Left(Message) (Pawn|GetControlledPawn) ActionValue))

(event Input|EnhancedActionEvents|EnhancedInputActionIA_MoveSpaceShip
  (params (ActionValue :type Float%20%28double-precision%29) (ElapsedSeconds :type Float%20%28double-precision%29) (TriggeredSeconds :type Float%20%28double-precision%29) (InputAction :type Input%20Action%20Object%20Reference :default "/Game/GameManager/Input_SpaceShip/IA_MoveSpaceShip.IA_MoveSpaceShip"))
  (bind _returnvalue (Pawn|GetControlledPawn))
  (:Triggered
    (Class|BPISpaceShip|MoveSpaceShip(Message) _returnvalue (> ActionValue 0.0)))
  (:Started
    (Class|BPISpaceShip|StartDeceleration(Message) _returnvalue false))
  (:Completed
    (Class|BPISpaceShip|StartDeceleration(Message) _returnvalue true)))

(event EventBeginPlay
  (Input|AddMappingContext (PlayerController|LocalPlayerSubsystems|GetEnhancedInputLocalPlayerSubsystem) "/Game/GameManager/Input_SpaceShip/IMC_Spaceship.IMC_Spaceship" 0 "(bIgnoreAllPressedKeysUntilRelease=True,bForceImmediately=False,bNotifyUserSettings=False)"))

(event Input|KeyboardEvents|Tab
  (params (Key :type Key%20Structure :default "None"))
  (:Pressed
    (bind _returnvalue (UserInterface|CreateWidget "/Game/QuestSystem/UI/W_QuestLog.W_QuestLog_C"))
    (UserInterface|Viewport|AddtoViewport _returnvalue 0)))

(fn ConstructionScript)