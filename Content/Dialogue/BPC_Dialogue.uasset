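; BPC_Dialogue is a dialogue component that shows and removes an on-screen dialogue display.
; ObjectInteracted creates a W_DialogueDisplay widget from the component's Name and Portrait, adds it to the viewport, and skips creation if one already exists.
; EndDialogue removes the widget and clears its reference.
; InteractWith and LookAt return empty strings, and BeginPlay and Tick are unused.
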(event Custom|CreateDialogueDisplay
  ;[0.15 0.15 0.15 0.5] Create Dialogue Display
  (Variables|Default|GetDialogueDisplay
    (:then)
    (:else
      (bind _returnvalue (UserInterface|CreateWidget "/Game/DialogueSystem/DialogueUI/W_DialogueDisplay.W_DialogueDisplay_C" 0 (Variables|Input|GetName) (Variables|Input|GetPortrait)))
      (bind _output_get (Variables|Default|SetDialogueDisplay _returnvalue))
      (UserInterface|Viewport|AddtoViewport _output_get 0))))

(event Custom|EndDialogue
  ;[0.15 0.15 0.15 0.5] End Dialogue Logic
  (bind _dialoguedisplay (Variables|Default|GetDialogueDisplay)
    (:then
      (Widget|RemovefromParent _dialoguedisplay)
      (Variables|Default|SetDialogueDisplay 0))
    (:else)))

(event EventBeginPlay)

(event EventTick
  (params (DeltaSeconds :type Float%20%28single-precision%29)))

(event EventObjectInteracted
  (params (Interactor :type Actor%20Object%20Reference))
  (CallFunction|CreateDialogueDisplay))

(fn Interactwith
  (return ""))

(fn Lookat
  (return ""))